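; Boss robot character that moves along a spline pathway while focusing on the player, armed with an attached knife and blowtorch.
; BeginPlay applies default GAS attributes, runs the boss behavior tree with the player as TargetActor, and spawns both weapons onto mesh sockets.
; Tick delegates movement to the first SplinePathway found while ShouldMove is set.
; Swipe restores the starting rotation before a delayed montage; death stops movement and AI logic.
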(event Custom|FindSpline
  (bind _outactors (Actor|GetAllActorsOfClass "/Game/_Game/Blueprints/AI/Boss/SplinePathway.SplinePathway_C"))
  (Variables|Default|SetSplinePoint (Utilities|Array|Get(acopy) _outactors)))

(event Custom|Swipe
  (Transformation|SetActorRotation (Variables|Default|GetDefaultRotation))
  (Utilities|FlowControl|Delay 1.0)
  (Animation|Montage|PlayMontage (Variables|Character|GetMesh) "/Game/_Game/Blueprints/AI/Boss/AM_Swipe.AM_Swipe"))

(event Custom|Spawn%20Knife%20And%20Attach
  ;[1 1 1] Spawn Weapon
  (bind _returnvalue (Game|SpawnActorfromClass "/Game/_Game/Blueprints/AI/Boss/Weapons/BP_BossKnife.BP_BossKnife_C" (Math|Transform|MakeTransform "0, 0, 0") "Undefined" 0 self))
  (bind _output_get (Variables|Default|SetKnifeRef _returnvalue))
  (Transformation|AttachComponentToComponent _output_get (Variables|Character|GetMesh) "KnifeSocket" "SnapToTarget" "SnapToTarget" "SnapToTarget" true)
  (bind _returnvalue_2 (Game|SpawnActorfromClass "/Game/_Game/Blueprints/AI/Boss/Weapons/BP_BossBlowTorch.BP_BossBlowTorch_C" (Math|Transform|MakeTransform "0, 0, 0") "Undefined" 0 self))
  (bind _output_get_2 (Variables|Default|SetBlowtorchRef _returnvalue_2))
  (Transformation|AttachComponentToComponent _output_get_2 (Variables|Character|GetMesh) "BlowtorchSocket" "SnapToTarget" "SnapToTarget" "SnapToTarget" true))

(event EventBeginPlay
  (bind _self self)
  (bind _returnvalue (AI|GetAIController _self))
  (|CallParentFunction)
  (Variables|Default|SetDefaultRotation (Transformation|GetActorRotation))
  (CallFunction|FindSpline)
  (GameplayEffects|ApplyGameplayEffectToSelf :self (Variables|Default|GetAbilitySystemComponent) :GameplayEffectClass "/Game/_Game/Blueprints/Abilities/GAS/GE_DefaultAttributes.GE_DefaultAttributes_C")
  (Utilities|IsValid _returnvalue
    (:Is%20Valid
      (AI|RunBehaviorTree _returnvalue "/Game/_Game/Blueprints/AI/Boss/Brains/BT_BossAI.BT_BossAI")
      (AI|Components|Blackboard|SetValueasObject (AI|GetBlackboard 0) (Utilities|Name|MakeLiteralName "TargetActor") (Game|GetPlayerCharacter 0))
      (CallFunction|SpawnKnifeandAttach))))

(event EventTick
  (params (DeltaSeconds :type Float%20%28single-precision%29))
  (if (Variables|Default|GetShouldMove)
    (bind _splinepoint (Variables|Default|GetSplinePoint)
      (:then
        (Class|BossSplineActor|MoveActor _splinepoint DeltaSeconds self (Game|GetPlayerCharacter 0) 0.5 2.0))
      (:else))))

(event EventHandleDeath
  (if (not (Class|BossAI|GetIsDead))
    (Class|BossAI|SetIsDeath true)
    (Variables|Default|SetShouldMove false)
    (AI|Logic|StopLogic (Variables|/Script/AIModule.AIController|GetBrainComponent (AI|GetAIController self)) "Dead")
    (Collision|SetCollisionEnabled (Variables|Character|GetMesh) "QueryOnly")))

(fn ConstructionScript)
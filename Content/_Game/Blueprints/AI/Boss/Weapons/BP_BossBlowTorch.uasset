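; Boss blowtorch weapon that applies a damage Gameplay Effect to the player while they are inside its capsule.
; BeginPlay caches the player character as BP_CharacterBase.
; Capsule begin overlap applies GE_BlowtorchDmg through that player's own Ability System Component, ignoring other actors.
; End overlap removes all stacks of the effect from the player, without checking which actor left.
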(event OnComponentBeginOverlap(Capsule)
  (params (OverlappedComponent :type Primitive%20Component%20Object%20Reference) (OtherActor :type Actor%20Object%20Reference) (OtherComp :type Primitive%20Component%20Object%20Reference) (OtherBodyIndex :type Integer) (bFromSweep :type Boolean) (SweepResult :type Hit%20Result%20Structure%20%28by%20ref%29))
  (bind _as_bp_character_base (Variables|Default|GetAs%20BP%20Character%20Base))
  (bind _returnvalue (Ability|GetAbilitySystemComponent _as_bp_character_base))
  (if (== OtherActor (Variables|Default|GetAs%20BP%20Character%20Base))
    (GameplayEffects|ApplyGameplayEffectToTarget :self _returnvalue :GameplayEffectClass "/Game/_Game/Blueprints/AI/Boss/Weapons/GE_BlowtorchDmg.GE_BlowtorchDmg_C" :Target _returnvalue)))

(event OnComponentEndOverlap(Capsule)
  (params (OverlappedComponent :type Primitive%20Component%20Object%20Reference) (OtherActor :type Actor%20Object%20Reference) (OtherComp :type Primitive%20Component%20Object%20Reference) (OtherBodyIndex :type Integer))
  (GameplayEffects|RemoveActiveGameplayEffectbySourceEffect (Ability|GetAbilitySystemComponent (Variables|Default|GetAs%20BP%20Character%20Base)) "/Game/_Game/Blueprints/AI/Boss/Weapons/GE_BlowtorchDmg.GE_BlowtorchDmg_C" 0 -1))

(event EventBeginPlay
  (bind _asbp_character_base (Utilities|Casting|CastToBP_CharacterBase (Game|GetPlayerCharacter 0)))
  (Variables|Default|SetAs%20BP%20Character%20Base _asbp_character_base))

(fn ConstructionScript)
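; BP_FallKnife is a boss weapon knife that damages the player through the Gameplay Ability System and destroys itself after a fixed lifetime.
; BeginPlay caches the player as BP_CharacterBase and starts the destroy timer.
; Any KnifeCapsule overlap applies GE_KnifeWeaponDmg to the cached player, using their ability system as both source and target.
; The overlap branch is always true, so what touched the knife is never checked.
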(event OnComponentBeginOverlap(KnifeCapsule)
  (params (OverlappedComponent :type Primitive%20Component%20Object%20Reference) (OtherActor :type Actor%20Object%20Reference) (OtherComp :type Primitive%20Component%20Object%20Reference) (OtherBodyIndex :type Integer) (bFromSweep :type Boolean) (SweepResult :type Hit%20Result%20Structure%20%28by%20ref%29))
  (bind _as_bp_character_base (Variables|Default|GetAs%20BP%20Character%20Base))
  (bind _returnvalue (Ability|GetAbilitySystemComponent _as_bp_character_base))
  (if true
    (GameplayEffects|ApplyGameplayEffectToTarget :self _returnvalue :GameplayEffectClass "/Game/_Game/Blueprints/AI/Boss/Weapons/GE_KnifeWeaponDmg.GE_KnifeWeaponDmg_C" :Target _returnvalue)))

(event Collision|EventActorBeginOverlap
  (params (OtherActor :type Actor%20Object%20Reference)))

(event EventTick
  (params (DeltaSeconds :type Float%20%28single-precision%29)))

(event EventBeginPlay
  (bind _asbp_character_base (Utilities|Casting|CastToBP_CharacterBase (Game|GetPlayerCharacter 0)))
  (Variables|Default|SetAs%20BP%20Character%20Base _asbp_character_base)
  (Utilities|FlowControl|Delay 12.0)
  (Actor|DestroyActor))

(fn ConstructionScript)
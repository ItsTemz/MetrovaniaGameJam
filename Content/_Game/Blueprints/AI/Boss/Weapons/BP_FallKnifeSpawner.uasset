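; Boss weapon spawner that drops a timed grid of BP_FallKnife actors, starting at its own location on BeginPlay.
; A custom delayed-loop macro fires one row of six knives every half second, stepping along Y until LoopInt reaches the row count.
; A helper macro spawns each knife at an offset from the spawner.
; The loop keeps ticking after the last row; older hand-placed delayed rows remain unconnected.
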(event EventBeginPlay
  (Utilities|ForLoopDelay 0 0 0.5 12
    (:Body
      (Utilities|NewMacro0 0.0 0.0)
      (Utilities|NewMacro0 1e+02 0.0)
      (Utilities|NewMacro0 2e+02 0.0)
      (Utilities|NewMacro0 3e+02 0.0)
      (Utilities|NewMacro0 4e+02 0.0)
      (Utilities|NewMacro0 5e+02 0.0)
      (bind _result (Math|Integer|IncrementInt (Variables|Default|Getloop%20int))
        (:%20%20
          (Variables|Default|Setloop%20int _result)
          (Variables|Default|SetY (+ (Variables|Default|GetY) 2e+02)))))))

(fn ConstructionScript)
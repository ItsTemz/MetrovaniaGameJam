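; BP_GruntAI is the grunt enemy character, an AI that fights with a projectile weapon.
; On BeginPlay it runs BT_GruntAI, sets default attributes and grants the projectile-fire ability through GAS, then spawns and equips BP_AIWeapon via its CombatComponent.
; FireProjectile triggers that ability.
; When health reaches zero it ragdolls, stops moving, ignores two trace channels and self-destroys after a delay, taking its weapon with it.
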(event Custom|On%20Health%20Changed
  (params (Value :type Float%20%28single-precision%29) (MaxValue :type Float%20%28single-precision%29))
  (bind _mesh (Variables|Character|GetMesh))
  (if (<= Value 0.0)
    (Input|DisableInput (Pawn|GetController) (Game|GetPlayerController 0))
    (Class|MICharacter|StartRagdoll)
    (AI|Navigation|StopMovement (AI|GetAIController self))
    (Collision|SetCollisionResponsetoChannel _mesh "ECC_GameTraceChannel1" "ECR_Ignore")
    (Collision|SetCollisionResponsetoChannel _mesh "ECC_GameTraceChannel2" "ECR_Ignore")
    (Utilities|FlowControl|Delay 5.0)
    (Actor|DestroyActor)))

(event Custom|InitEnemy
  (GameplayEffects|ApplyGameplayEffectToSelf :self (Variables|Default|GetAbilitySystemComponent) :GameplayEffectClass "/Game/_Game/Blueprints/Abilities/GAS/GE_DefaultAttributes.GE_DefaultAttributes_C")
  (Class|CharacterBase|GiveAbility "/Game/_Game/Blueprints/Abilities/SkeeBall/GA_AI_ProjectileFire.GA_AI_ProjectileFire_C")
  (EventDispatchers|BindEventtoOnHealthChanged (Variables|Default|GetAttributeSet) (delegate Custom|On%20Health%20Changed)))

(event Custom|FireProjectile
  (Abilities|TryActivateAbilitybyClass (Variables|Default|GetAbilitySystemComponent) "/Game/_Game/Blueprints/Abilities/SkeeBall/GA_AI_ProjectileFire.GA_AI_ProjectileFire_C" true))

(event EventDestroyed
  (Actor|DestroyActor (Variables|/Script/MetroidvaniaJam17.CombatComponent|GetEquippedWeapon (Variables|Default|GetCombatComponent)))
  (|CallParentFunction))

(event EventBeginPlay
  (bind _self self)
  (bind _returnvalue (AI|GetAIController _self))
  (Utilities|IsValid _returnvalue
    (:Is%20Valid
      (AI|RunBehaviorTree _returnvalue "/Game/_Game/Blueprints/AI/Enemies/BT_GruntAI.BT_GruntAI")
      (CallFunction|InitEnemy)
      (bind _returnvalue_2 (Game|SpawnActorfromClass "/Game/_Game/Blueprints/Weapons/BP_AIWeapon.BP_AIWeapon_C" (Math|Transform|MakeTransform "0, 0, 0") "Undefined" 0 0))
      (Class|CombatComponent|ChangeWeapon (Variables|Default|GetCombatComponent) _returnvalue_2)
      (|CallParentFunction))))

(fn ConstructionScript)
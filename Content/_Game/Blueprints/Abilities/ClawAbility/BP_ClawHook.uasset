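; BP_ClawHook is the projectile actor for the claw ability's hook.
; On BeginPlay it applies its Velocity to the ProjectileMovement component and records its start location.
; If a valid HomingTarget is set, it homes onto that actor's root component; otherwise it flies without homing.
; Each tick it destroys itself once its straight-line distance from the start reaches MaxDistance.
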(event EventBeginPlay
  (bind _projectilemovement (Variables|Default|GetProjectileMovement))
  (Variables|/Script/Engine.MovementComponent|SetVelocity (Variables|Default|GetProjectileMovement) (Variables|Default|GetVelocity))
  (Variables|Default|SetStartLocation (Transformation|GetActorLocation))
  (bind _homingtarget (Variables|Default|GetHomingTarget)
    (:then
      (Variables|/Script/Engine.ProjectileMovementComponent|SetbIsHomingProjectile _projectilemovement true)
      (Variables|/Script/Engine.ProjectileMovementComponent|SetHomingTargetComponent _projectilemovement (Variables|/Script/Engine.Actor|GetRootComponent _homingtarget)))
    (:else
      (Variables|/Script/Engine.ProjectileMovementComponent|SetbIsHomingProjectile _projectilemovement false))))

(event EventTick
  (params (DeltaSeconds :type Float%20%28single-precision%29))
  (if (>= (Math|Vector|Distance(Vector) (Variables|Default|GetStartLocation) (Transformation|GetActorLocation)) (Variables|Default|GetMaxDistance))
    (Actor|DestroyActor)))

(fn ConstructionScript)
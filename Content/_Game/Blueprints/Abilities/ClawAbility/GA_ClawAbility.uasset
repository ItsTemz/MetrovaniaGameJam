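; Gameplay ability for the claw, which toggles the character's GrappleComponent: it cancels an active grapple or fires a new one, provided a weapon is equipped.
; The grapple aims at the CombatComponent's current target, otherwise at an object hit under the cursor, with low hit points raised in Z.
; The ability ends after each action or without a weapon, but stays active when neither target nor cursor hit exists.
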(event Ability|EventActivateAbility
  (bind (_character _equipped_weapon) (CallFunction|GetCharacter))
  (Utilities|IsValid _equipped_weapon
    (:Is%20Valid
      (if (Default|IsinUse? (Variables|/Game/_Game/Blueprints/BP_CharacterBase.BP_CharacterBase_C|GetGrappleComponent _character))
        (Default|CancelGrapple (Variables|/Game/_Game/Blueprints/BP_CharacterBase.BP_CharacterBase_C|GetGrappleComponent _character))
        (Ability|EndAbility)
        (else
          (bind _currenttarget (Variables|/Script/MetroidvaniaJam17.CombatComponent|GetCurrentTarget (Variables|/Script/MetroidvaniaJam17.CharacterBase|GetCombatComponent _character))
            (:then
              (Default|FireGrapple (Variables|/Game/_Game/Blueprints/BP_CharacterBase.BP_CharacterBase_C|GetGrappleComponent _character) (Transformation|GetActorLocation _currenttarget) "0.000000,40.000000, 0")
              (Ability|EndAbility :!label _label))
            (:else
              (if (.ReturnValue (Class|PlayerController|GetHitResultUnderCursorforObjects (Variables|/Script/MoveIt.MICharacter_TwinStick|GetPlayerController _character) (Utilities|Array|MakeArray "ObjectTypeQuery1" "ObjectTypeQuery2" "ObjectTypeQuery8") true))
                (Default|FireGrapple (Variables|/Game/_Game/Blueprints/BP_CharacterBase.BP_CharacterBase_C|GetGrappleComponent _character) (select (.ReturnValue (Class|PlayerController|GetHitResultUnderCursorforObjects (Variables|/Script/MoveIt.MICharacter_TwinStick|GetPlayerController _character) (Utilities|Array|MakeArray "ObjectTypeQuery1" "ObjectTypeQuery2" "ObjectTypeQuery8") true)) (select (> (.Z (Math|Vector|BreakVector (.ImpactPoint (Collision|BreakHitResult (.HitResult (Class|PlayerController|GetHitResultUnderCursorforObjects (Variables|/Script/MoveIt.MICharacter_TwinStick|GetPlayerController _character) (Utilities|Array|MakeArray "ObjectTypeQuery1" "ObjectTypeQuery2" "ObjectTypeQuery8") true)))))) 5e+01) (.Location (Collision|BreakHitResult (.HitResult (Class|PlayerController|GetHitResultUnderCursorforObjects (Variables|/Script/MoveIt.MICharacter_TwinStick|GetPlayerController _character) (Utilities|Array|MakeArray "ObjectTypeQuery1" "ObjectTypeQuery2" "ObjectTypeQuery8") true)))) (Math|Vector|MakeVector (.X (Math|Vector|BreakVector (.ImpactPoint (Collision|BreakHitResult (.HitResult (Class|PlayerController|GetHitResultUnderCursorforObjects (Variables|/Script/MoveIt.MICharacter_TwinStick|GetPlayerController _character) (Utilities|Array|MakeArray "ObjectTypeQuery1" "ObjectTypeQuery2" "ObjectTypeQuery8") true)))))) (.Y (Math|Vector|BreakVector (.ImpactPoint (Collision|BreakHitResult (.HitResult (Class|PlayerController|GetHitResultUnderCursorforObjects (Variables|/Script/MoveIt.MICharacter_TwinStick|GetPlayerController _character) (Utilities|Array|MakeArray "ObjectTypeQuery1" "ObjectTypeQuery2" "ObjectTypeQuery8") true)))))) (+ (.Z (Math|Vector|BreakVector (.ImpactPoint (Collision|BreakHitResult (.HitResult (Class|PlayerController|GetHitResultUnderCursorforObjects (Variables|/Script/MoveIt.MICharacter_TwinStick|GetPlayerController _character) (Utilities|Array|MakeArray "ObjectTypeQuery1" "ObjectTypeQuery2" "ObjectTypeQuery8") true)))))) 1e+02))) (.TraceEnd (Collision|BreakHitResult (.HitResult (Class|PlayerController|GetHitResultUnderCursorforObjects (Variables|/Script/MoveIt.MICharacter_TwinStick|GetPlayerController _character) (Utilities|Array|MakeArray "ObjectTypeQuery1" "ObjectTypeQuery2" "ObjectTypeQuery8") true))))) "0.000000,40.000000, 0")
                (goto _label)))))))
    (:Is%20Not%20Valid
      (Ability|EndAbility))))

(event Ability|EventOnEndAbility
  (params (bWasCancelled :type Boolean)))
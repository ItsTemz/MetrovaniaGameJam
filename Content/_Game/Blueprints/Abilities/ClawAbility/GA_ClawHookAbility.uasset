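; Gameplay ability that fires or cancels the character's claw grapple hook, provided a weapon is equipped.
; If the GrappleComponent is already in use, activation cancels the grapple.
; Otherwise it fires at the CombatComponent's current target, or at the hit or end point of a forward camera trace against static world objects.
; The ability ends immediately after each action, leaving the grapple itself to the component.
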(event Ability|EventActivateAbility
  (bind (_character _equipped_weapon) (CallFunction|GetCharacter))
  (Utilities|IsValid _equipped_weapon
    (:Is%20Valid
      (if (Default|IsinUse? (Variables|/Game/_Game/Blueprints/BP_CharacterBase.BP_CharacterBase_C|GetGrappleComponent _character))
        (Default|CancelGrapple (Variables|/Game/_Game/Blueprints/BP_CharacterBase.BP_CharacterBase_C|GetGrappleComponent _character))
        (Ability|EndAbility)
        (else
          (bind _currenttarget (Variables|/Script/MetroidvaniaJam17.CombatComponent|GetCurrentTarget (Variables|/Script/MetroidvaniaJam17.CharacterBase|GetCombatComponent _character))
            (:then
              (Default|FireGrapple (Variables|/Game/_Game/Blueprints/BP_CharacterBase.BP_CharacterBase_C|GetGrappleComponent _character) (Transformation|GetActorLocation _currenttarget) "0.000000,40.000000, 0"))
            (:else
              (bind _outhit (Collision|LineTraceForObjects (Transformation|GetWorldLocation (Class|MIViewComponent|GetCurrentCamera (Variables|/Script/MetroidvaniaJam17.CharacterBase|GetViewComponent _character))) (+ (Transformation|GetWorldLocation (Class|MIViewComponent|GetCurrentCamera (Variables|/Script/MetroidvaniaJam17.CharacterBase|GetViewComponent _character))) (* (Math|Vector|GetForwardVector (Transformation|GetWorldRotation (Class|MIViewComponent|GetCurrentCamera (Variables|/Script/MetroidvaniaJam17.CharacterBase|GetViewComponent _character)))) 2e+03)) (Utilities|Array|MakeArray "ObjectTypeQuery1") false (Utilities|Array|MakeArray _character _equipped_weapon) "None"))
              (Default|FireGrapple (Variables|/Game/_Game/Blueprints/BP_CharacterBase.BP_CharacterBase_C|GetGrappleComponent _character) (select (.bBlockingHit (Collision|BreakHitResult _outhit)) (.ImpactPoint (Collision|BreakHitResult _outhit)) (.TraceEnd (Collision|BreakHitResult _outhit))) "0.000000,40.000000, 0")))
          (Ability|EndAbility))))
    (:Is%20Not%20Valid
      (Ability|EndAbility))))
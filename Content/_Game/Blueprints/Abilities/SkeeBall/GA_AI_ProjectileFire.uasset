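; Gameplay ability that makes a Grunt AI fire a projectile from its equipped weapon.
; On activation it commits, starts the fire montage and proceeds immediately without waiting for the montage to finish.
; It traces forward from the current view camera against world-static objects and passes the impact point, or trace end, to the weapon as a non-homing target.
; It ends after firing, but never explicitly ends if the cast or weapon check fails.
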(event Ability|EventActivateAbility
  (Ability|CommitAbility)
  (|PlayMontageandWaitProxy "None" "/Game/_Game/Blueprints/Abilities/SkeeBall/AM_Fire.AM_Fire" 1.0 "None" true 1.0 0.0
    (:then
      (bind _asbp_grunt_ai (Utilities|Casting|CastToBP_GruntAI (Ability|GetOwningActorfromActorInfo)))
      (bind _equippedweapon (Variables|/Script/MetroidvaniaJam17.CombatComponent|GetEquippedWeapon (Variables|/Script/MetroidvaniaJam17.CharacterBase|GetCombatComponent _asbp_grunt_ai))
        (:then
          (bind _outhit (Collision|LineTraceForObjects (Transformation|GetWorldLocation (Class|MIViewComponent|GetCurrentCamera (Variables|/Script/MetroidvaniaJam17.CharacterBase|GetViewComponent _asbp_grunt_ai))) (+ (Transformation|GetWorldLocation (Class|MIViewComponent|GetCurrentCamera (Variables|/Script/MetroidvaniaJam17.CharacterBase|GetViewComponent _asbp_grunt_ai))) (* (Math|Vector|GetForwardVector (Transformation|GetWorldRotation (Class|MIViewComponent|GetCurrentCamera (Variables|/Script/MetroidvaniaJam17.CharacterBase|GetViewComponent _asbp_grunt_ai)))) 2e+03)) (Utilities|Array|MakeArray "ObjectTypeQuery1") false (Utilities|Array|MakeArray _asbp_grunt_ai _equippedweapon) "None"))
          (Class|Weapon|Fire _equippedweapon (select (.bBlockingHit (Collision|BreakHitResult _outhit)) (.ImpactPoint (Collision|BreakHitResult _outhit)) (.TraceEnd (Collision|BreakHitResult _outhit))) false)
          (Ability|EndAbility))
        (:else)))))
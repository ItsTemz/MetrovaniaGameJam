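; Gameplay ability that fires the character's equipped weapon as a projectile attack.
; It commits, starts the fire montage and fires immediately, homing on the combat component's current target.
; With no target, or one carrying a grapple-swing component, it fires unhomed at a camera-forward line trace against static world objects, using the impact or trace end.
; The ability ends right after firing, but has no end path when no weapon is equipped.
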(event Ability|EventActivateAbility
  (Ability|CommitAbility)
  (|PlayMontageandWaitProxy "None" "/Game/_Game/Blueprints/Abilities/SkeeBall/AM_Fire.AM_Fire" 1.0 "None" true 1.0 0.0
    (:then
      (bind (_character _equipped_weapon) (CallFunction|GetCharacter))
      (Utilities|IsValid _equipped_weapon
        (:Is%20Valid
          (bind _currenttarget (Variables|/Script/MetroidvaniaJam17.CombatComponent|GetCurrentTarget (Variables|/Script/MetroidvaniaJam17.CharacterBase|GetCombatComponent _character))
            (:then
              (Utilities|IsValid (Actor|GetComponentbyClass _currenttarget "/Game/_Game/Blueprints/Abilities/ClawAbility/BP_GrappleSwing.BP_GrappleSwing_C")
                (:Is%20Valid
                  (bind _outhit (Collision|LineTraceForObjects (Transformation|GetWorldLocation (Class|MIViewComponent|GetCurrentCamera (Variables|/Script/MetroidvaniaJam17.CharacterBase|GetViewComponent _character))) (+ (Transformation|GetWorldLocation (Class|MIViewComponent|GetCurrentCamera (Variables|/Script/MetroidvaniaJam17.CharacterBase|GetViewComponent _character))) (* (Math|Vector|GetForwardVector (Transformation|GetWorldRotation (Class|MIViewComponent|GetCurrentCamera (Variables|/Script/MetroidvaniaJam17.CharacterBase|GetViewComponent _character)))) 2e+03)) (Utilities|Array|MakeArray "ObjectTypeQuery1") false (Utilities|Array|MakeArray _character _equipped_weapon) "None" :!label _label))
                  (Class|Weapon|Fire _equipped_weapon (select (.bBlockingHit (Collision|BreakHitResult _outhit)) (.ImpactPoint (Collision|BreakHitResult _outhit)) (.TraceEnd (Collision|BreakHitResult _outhit))) false))
                (:Is%20Not%20Valid
                  (Class|Weapon|Fire _equipped_weapon (Transformation|GetActorLocation _currenttarget) true))))
            (:else
              (goto _label)))
          (Ability|EndAbility))))))

(event Ability|EventOnEndAbility
  (params (bWasCancelled :type Boolean)))
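; GA_TennisBall is a SkeeBall gameplay ability whose ActivateAbility event is empty, so its firing logic never runs.
; The disconnected chain plays AM_Fire and fires the equipped weapon with homing at the combat target, raised above its origin.
; Without a target, it fires unhomed above the WorldStatic point under the cursor.
; The ability ends after firing or when the montage blends out, is interrupted or is cancelled.
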(event Ability|EventActivateAbility)
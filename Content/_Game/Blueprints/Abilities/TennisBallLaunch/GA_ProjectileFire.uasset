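; Gameplay ability that plays a fire montage and fires the character's equipped weapon as soon as the montage starts, then ends.
; With a valid combat target, it fires a homing shot slightly above the target's location.
; Otherwise, it fires without homing at a debug-drawn WorldStatic trace's hit or end point; that end scales location plus forward vector together.
; Montage blend-out, interruption or cancellation also ends the ability.
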(event Ability|EventActivateAbility
  (|PlayMontageandWaitProxy "None" "/Game/_Game/Blueprints/Abilities/TennisBallLaunch/AM_Fire.AM_Fire" 1.0 "None" true 1.0 0.0
    (:then
      (bind (_character _equipped_weapon) (CallFunction|GetCharacter))
      (Utilities|IsValid _equipped_weapon
        (:Is%20Valid
          (bind _currenttarget (Variables|/Script/MetroidvaniaJam17.CombatComponent|GetCurrentTarget (Variables|/Script/MetroidvaniaJam17.CharacterBase|GetCombatComponent _character))
            (:then
              (Class|Weapon|Fire _equipped_weapon (+ (Transformation|GetActorLocation _currenttarget) "0,0,100.000000") true)
              (Ability|EndAbility :!label _label))
            (:else
              (bind _outhit (Collision|LineTraceForObjects (Transformation|GetActorLocation _character) (* (+ (Transformation|GetActorLocation _character) (Transformation|GetActorForwardVector _character)) 2e+03) (Utilities|Array|MakeArray "ObjectTypeQuery1") false (Utilities|Array|MakeArray _character _equipped_weapon) "ForDuration"))
              (if true
                (Class|Weapon|Fire _equipped_weapon (select (.bBlockingHit (Collision|BreakHitResult _outhit)) (.Location (Collision|BreakHitResult _outhit)) (.TraceEnd (Collision|BreakHitResult _outhit))) false)
                (goto _label)))))))
    (:OnBlendOut
      (Ability|EndAbility :!label _label_2))
    (:OnInterrupted
      (goto _label_2))
    (:OnCancelled
      (goto _label_2))))
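; Gameplay ability for the tennis ball launch, which plays a fire montage and fires the character's equipped weapon as the montage starts.
; With a current combat target, the shot homes on a point raised above that target.
; Otherwise it fires unguided at a raised point on the WorldStatic surface under the cursor.
; The ability ends right after firing, or when the montage blends out or is interrupted or cancelled.
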(event Ability|EventActivateAbility
  (|PlayMontageandWaitProxy "None" "/Game/_Game/Blueprints/Abilities/TennisBallLaunch/AM_Fire.AM_Fire" 1.0 "None" true 1.0 0.0
    (:then
      (bind (_character _equipped_weapon) (CallFunction|GetCharacter))
      (Utilities|IsValid _equipped_weapon
        (:Is%20Valid
          (bind _currenttarget (Variables|/Script/MetroidvaniaJam17.CombatComponent|GetCurrentTarget (Variables|/Script/MetroidvaniaJam17.CharacterBase|GetCombatComponent _character))
            (:then
              (Class|Weapon|Fire _equipped_weapon (+ (Transformation|GetActorLocation _currenttarget) "0,0,100.000000") true)
              (Ability|EndAbility :!label _label))
            (:else
              (if (.ReturnValue (Class|PlayerController|GetHitResultUnderCursorforObjects (Variables|/Script/MoveIt.MICharacter_TwinStick|GetPlayerController _character) (Utilities|Array|MakeArray "ObjectTypeQuery1") true))
                (Class|Weapon|Fire _equipped_weapon (Math|Vector|MakeVector (.X (Math|Vector|BreakVector (.Location (Collision|BreakHitResult (.HitResult (Class|PlayerController|GetHitResultUnderCursorforObjects (Variables|/Script/MoveIt.MICharacter_TwinStick|GetPlayerController _character) (Utilities|Array|MakeArray "ObjectTypeQuery1") true)))))) (.Y (Math|Vector|BreakVector (.Location (Collision|BreakHitResult (.HitResult (Class|PlayerController|GetHitResultUnderCursorforObjects (Variables|/Script/MoveIt.MICharacter_TwinStick|GetPlayerController _character) (Utilities|Array|MakeArray "ObjectTypeQuery1") true)))))) (+ (.Z (Math|Vector|BreakVector (.Location (Collision|BreakHitResult (.HitResult (Class|PlayerController|GetHitResultUnderCursorforObjects (Variables|/Script/MoveIt.MICharacter_TwinStick|GetPlayerController _character) (Utilities|Array|MakeArray "ObjectTypeQuery1") true)))))) 1e+02)) false)
                (goto _label)))))))
    (:OnBlendOut
      (Ability|EndAbility :!label _label_2))
    (:OnInterrupted
      (goto _label_2))
    (:OnCancelled
      (goto _label_2))))
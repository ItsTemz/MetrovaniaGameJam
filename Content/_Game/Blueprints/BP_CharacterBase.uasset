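; Base character Blueprint with Gameplay Ability System abilities, automatic soft targeting and ragdoll death.
; BeginPlay applies default attributes and grants the claw hook and projectile abilities, which input actions activate, while zero health triggers ragdoll and delayed destruction.
; Each tick, a sphere overlap picks the TargetComponent actor best aligned with camera forward within a cone, updating CombatComponent and an attached marker.
; Jump and landing events drive CameraBoom; IsLockedOnToTarget is an empty stub.
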(event Custom|On%20Health%20Changed
  (params (Value :type Float%20%28single-precision%29) (MaxValue :type Float%20%28single-precision%29))
  (if (<= Value 0.0)
    (Class|MICharacter|StartRagdoll)
    (Utilities|FlowControl|Delay 5.0)
    (Actor|DestroyActor)))

(event EventOnJumped
  (Class|MISpringArmComponent|OnCharacterJumped (Variables|Default|GetCameraBoom)))

(event EventTick
  (params (DeltaSeconds :type Float%20%28single-precision%29))
  ;[0.6406 0.02183 1] Targeting
  (bind _currenttarget (CallFunction|FindBestTarget))
  (CallFunction|SetCurrentTarget _currenttarget))

(event EventBeginPlay
  (Class|CombatComponent|SetActionMode (Variables|Default|GetCombatComponent) "EAM_AdventureMode")
  (GameplayEffects|ApplyGameplayEffectToSelf :self (Variables|Default|GetAbilitySystemComponent) :GameplayEffectClass "/Game/_Game/Blueprints/Abilities/GAS/GE_DefaultAttributes.GE_DefaultAttributes_C")
  (Class|CharacterBase|GiveAbility "/Game/_Game/Blueprints/Abilities/ClawAbility/GA_ClawHookAbility.GA_ClawHookAbility_C")
  (Class|CharacterBase|GiveAbility "/Game/_Game/Blueprints/Abilities/SkeeBall/GA_ProjectileFire.GA_ProjectileFire_C")
  (EventDispatchers|BindEventtoOnHealthChanged (Variables|Default|GetAttributeSet) (delegate Custom|On%20Health%20Changed)))

(event EventOnLanded
  (params (Hit :type Hit%20Result%20Structure%20%28by%20ref%29))
  (Class|MISpringArmComponent|OnCharacterLanded (Variables|Default|GetCameraBoom) 1e+01))

(event Input|ActionEvents|InputActionFireBall
  (params (Key :type Key%20Structure :default "None"))
  (:Pressed
    (Abilities|TryActivateAbilitybyClass (Variables|Default|GetAbilitySystemComponent) "/Game/_Game/Blueprints/Abilities/SkeeBall/GA_ProjectileFire.GA_ProjectileFire_C" true)))

(event Input|ActionEvents|InputActionFireClaw
  (params (Key :type Key%20Structure :default "None"))
  (:Pressed
    (Abilities|TryActivateAbilitybyClass (Variables|Default|GetAbilitySystemComponent) "/Game/_Game/Blueprints/Abilities/ClawAbility/GA_ClawHookAbility.GA_ClawHookAbility_C" true)))

(fn ConstructionScript)

(fn FindBestTarget
  (bind _adventurecamera (Variables|Default|GetAdventureCamera))
  ;[1 1 1] Check For Actors in a sphere
  (bind _outactors (Collision|SphereOverlapActors (Transformation|GetActorLocation) (Variables|Default|GetTargetingRange) (Utilities|Array|MakeArray "ObjectTypeQuery1" "ObjectTypeQuery3" "ObjectTypeQuery8" "ObjectTypeQuery2") "/Script/Engine.Actor" (Utilities|Array|MakeArray self)))
  (for _array_element _outactors
    ;[1 1 1] Check if those Actors are Targetable
    (bind _output_get (LocalVariables|SetCurrentTargetLocal _array_element))
    (Utilities|IsValid (Actor|GetComponentbyClass _output_get "/Script/MetroidvaniaJam17.TargetComponent")
      (:Is%20Valid
        ;[1 1 1] Set the closest actor
        (bind _output_get_2 (LocalVariables|SetCurrentValueLocal (Math|Vector|DotProduct (Math|Vector|GetForwardVector _adventurecamera) (Math|Vector|GetUnitDirection(Vector) (Transformation|GetWorldLocation _adventurecamera) (Transformation|GetActorLocation (LocalVariables|GetCurrentTargetLocal))))))
        (if (or (> _output_get_2 (LocalVariables|GetBestValueLocal)) (not (Utilities|IsValid (LocalVariables|GetBestTargetLocal))))
          (LocalVariables|SetBestValueLocal (LocalVariables|GetCurrentValueLocal))
          (LocalVariables|SetBestTargetLocal (LocalVariables|GetCurrentTargetLocal))))))
  (LocalVariables|GetBestTargetLocal
    (:then
      (if (<= (Class|KismetMathLibrary|DegAcos (LocalVariables|GetBestValueLocal)) (Variables|Default|GetTargetingConeAngle))
        (return (LocalVariables|GetBestTargetLocal))
        (else
          (return 0))))
    (:else
      (return 0))))

(fn SetCurrentTarget
  (params (Target :type Actor%20Object%20Reference))
  (if (!= Target (Variables|Default|GetCurrentTarget))
    (Utilities|FlowControl|Sequence
      (:then_0
        (CallFunction|EndTarget))
      (:then_1
        (bind _output_get (Variables|Default|SetCurrentTarget Target))
        (Variables|/Script/MetroidvaniaJam17.CombatComponent|SetCurrentTarget (Variables|Default|GetCombatComponent) _output_get))
      (:then_2
        (CallFunction|BeginTarget)))))

(fn EndTarget
  (bind _targetmarker (Variables|Default|GetTargetMarker)
    (:then
      (Actor|DestroyActor _targetmarker)
      (Variables|Default|SetTargetMarker 0))
    (:else)))

(fn BeginTarget
  (bind _currenttarget (Variables|Default|GetCurrentTarget)
    (:then
      (bind _returnvalue (Game|SpawnActorfromClass "/Game/_Game/Blueprints/Targeting/BP_TargetActor.BP_TargetActor_C" (Math|Transform|MakeTransform (Transformation|GetActorLocation _currenttarget) "0, 0, 0" "1.000000,1.000000,1.000000") "Undefined" 0 0))
      (bind _output_get (Variables|Default|SetTargetMarker _returnvalue))
      (Transformation|AttachActorToActor _output_get (Variables|Default|GetCurrentTarget) "TargetSocket" "SnapToTarget" "SnapToTarget" "SnapToTarget" true))
    (:else)))

(fn IsLockedontoTarget)
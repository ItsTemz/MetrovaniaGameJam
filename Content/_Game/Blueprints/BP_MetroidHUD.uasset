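; BP_MetroidHUD is a HUD-named Blueprint holding main menu show and dismiss logic that is currently disconnected.
; BeginPlay and StartGame are empty, so neither chain runs.
; One orphaned chain creates WBP_Menu and switches to UI-only input with the cursor shown.
; The other removes the menu, restores game input, hides the cursor and blends the view to the player pawn.
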(event Custom|Start%20Game)

(event EventBeginPlay)

(fn ConstructionScript)
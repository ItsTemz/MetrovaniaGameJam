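; BP_BossBlowTorch is an unfinished boss blowtorch weapon that probes for targets in front of its barrel.
; Every tick, with no working on/off toggle yet, it sphere-traces forward from TorchBarrel on the Visibility channel using FireRadius, with debug drawing.
; BeginPlay caches the player character, but the hit comparison against it is unconnected, so the trace has no gameplay effect.
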(event EventBeginPlay
  (bind _asbp_character_base (Utilities|Casting|CastToBP_CharacterBase (Game|GetPlayerCharacter 0)))
  (Variables|Default|SetAs%20BP%20Character%20Base _asbp_character_base))

(event EventTick
  (params (DeltaSeconds :type Float%20%28single-precision%29))
  (bind _torchbarrel (Variables|Default|GetTorchBarrel))
  (bind _returnvalue (Transformation|GetWorldLocation _torchbarrel))
  ;[1 1 1] make a bool for turning torch on and off
  (if true
    ;[1 1 1] debug mode on
    (bind _outhit (Collision|SphereTraceByChannel _returnvalue (+ _returnvalue (* (Math|Vector|GetForwardVector _torchbarrel) 1e+03)) (Variables|Default|GetFire%20Radius) "TraceTypeQuery1" false 0 "ForDuration"))))

(fn ConstructionScript)
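; BP_BossTest is a test boss enemy that walks a fixed patrol loop.
; BeginPlay calls the parent, then chains four AIMoveTo nodes through hardcoded world positions, with the last success wiring back to the first.
; Only the success outputs are connected, so a failed move ends the patrol.
; It adds no other active logic of its own.
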(event EventBeginPlay
  (bind _self self)
  (|CallParentFunction)
  (AI|AIMoveTo _self "3700.000000,910.000000,72.000000" 0 5.0 false :!label _label
    (:OnSuccess
      (AI|AIMoveTo _self "3700.000000,1620.000000,72.000000" 0 5.0 false
        (:OnSuccess
          (AI|AIMoveTo self "3010.000000,1620.000000,72.000000" 0 5.0 false
            (:OnSuccess
              (AI|AIMoveTo self "3010.000000,680.000000,72.000000" 0 5.0 false
                (:OnSuccess
                  (goto _label))))))))))

(event Collision|EventActorBeginOverlap
  (params (OtherActor :type Actor%20Object%20Reference)))

(event EventTick
  (params (DeltaSeconds :type Float%20%28single-precision%29))
  (|CallParentFunction DeltaSeconds) ; This node is disabled and will not be called.\nDrag off pins to build functionality.
)

(fn ConstructionScript
  (|CallParentFunction))
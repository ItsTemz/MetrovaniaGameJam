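; Jukebox interactable whose music the player toggles and hears fade by proximity.
; BeginPlay starts MusicAudio paused and caches the player's CharacterBase.
; Interact alternates between unpausing and pausing the music through a FlipFlop.
; AreaBox overlaps with that cached character call a short FadeIn on entry and FadeOut on exit.
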(event OnComponentEndOverlap(AreaBox)
  (params (OverlappedComponent :type Primitive%20Component%20Object%20Reference) (OtherActor :type Actor%20Object%20Reference) (OtherComp :type Primitive%20Component%20Object%20Reference) (OtherBodyIndex :type Integer))
  (if (== OtherActor (Variables|Default|GetCharacter))
    (Audio|Components|Audio|FadeOut (Variables|Default|GetMusicAudio) 0.3 0.0 "Linear" :!class /Script/Engine.AudioComponent)))

(event OnComponentBeginOverlap(AreaBox)
  (params (OverlappedComponent :type Primitive%20Component%20Object%20Reference) (OtherActor :type Actor%20Object%20Reference) (OtherComp :type Primitive%20Component%20Object%20Reference) (OtherBodyIndex :type Integer) (bFromSweep :type Boolean) (SweepResult :type Hit%20Result%20Structure%20%28by%20ref%29))
  (if (== OtherActor (Variables|Default|GetCharacter))
    (Audio|Components|Audio|FadeIn (Variables|Default|GetMusicAudio) 0.3 1.0 0.0 "Linear" :!class /Script/Engine.AudioComponent)))

(event EventBeginPlay
  (|CallParentFunction)
  (Class|AudioComponent|SetPaused (Variables|Default|GetMusicAudio) true)
  (bind _ascharacter_base (Utilities|Casting|CastToCharacterBase (Game|GetPlayerCharacter 0)))
  (Variables|Default|SetCharacter _ascharacter_base))

(event Collision|EventActorBeginOverlap
  (params (OtherActor :type Actor%20Object%20Reference))
  (|CallParentFunction OtherActor) ; This node is disabled and will not be called.\nDrag off pins to build functionality.
)

(event EventTick
  (params (DeltaSeconds :type Float%20%28single-precision%29))
  (|CallParentFunction DeltaSeconds) ; This node is disabled and will not be called.\nDrag off pins to build functionality.
)

(event EventInteract
  (Utilities|FlowControl|FlipFlop
    (:A
      (Class|AudioComponent|SetPaused (Variables|Default|GetMusicAudio) false))
    (:B
      (Class|AudioComponent|SetPaused (Variables|Default|GetMusicAudio) true))))

(fn ConstructionScript
  (|CallParentFunction))
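; BP_DinerDoor is an automatic double door for the diner that swings open when a character approaches.
; A Box overlap with any BP_CharacterBase plays the Open timeline, and end overlap reverses it.
; The timeline alpha lerps each leaf's relative rotation up to a quarter turn, with the left leaf negated to mirror the right.
; End overlap does not check whether other characters remain inside the box.
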(event OnComponentBeginOverlap(Box)
  (params (OverlappedComponent :type Primitive%20Component%20Object%20Reference) (OtherActor :type Actor%20Object%20Reference) (OtherComp :type Primitive%20Component%20Object%20Reference) (OtherBodyIndex :type Integer) (bFromSweep :type Boolean) (SweepResult :type Hit%20Result%20Structure%20%28by%20ref%29))
  (Utilities|Casting|CastToBP_CharacterBase OtherActor)
  (bind _openalpha (Timeline|Open Play)
    (:Update
      (Utilities|FlowControl|Sequence
        (:then_0
          (Transformation|SetRelativeRotation (Variables|Default|GetSM_DinerDoorRight) (Math|Rotator|Lerp(Rotator) "0, 0, 0" "0,90.000000, 0" _openalpha) false false))
        (:then_1
          (Transformation|SetRelativeRotation (Variables|Default|GetSM_DinerDoorLeft) (* (Math|Rotator|Lerp(Rotator) "0, 0, 0" "0,90.000000, 0" _openalpha) -1.0) false false))))))

(event OnComponentEndOverlap(Box)
  (params (OverlappedComponent :type Primitive%20Component%20Object%20Reference) (OtherActor :type Actor%20Object%20Reference) (OtherComp :type Primitive%20Component%20Object%20Reference) (OtherBodyIndex :type Integer))
  (Utilities|Casting|CastToBP_CharacterBase OtherActor)
  (bind _openalpha (Timeline|Open Reverse)
    (:Update
      (Utilities|FlowControl|Sequence
        (:then_0
          (Transformation|SetRelativeRotation (Variables|Default|GetSM_DinerDoorRight) (Math|Rotator|Lerp(Rotator) "0, 0, 0" "0,90.000000, 0" _openalpha) false false))
        (:then_1
          (Transformation|SetRelativeRotation (Variables|Default|GetSM_DinerDoorLeft) (* (Math|Rotator|Lerp(Rotator) "0, 0, 0" "0,90.000000, 0" _openalpha) -1.0) false false))))))

(fn ConstructionScript)
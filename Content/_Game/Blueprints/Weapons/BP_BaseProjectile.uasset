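; BP_BaseProjectile is a base projectile that delivers a Gameplay Effect to what it hits through the Gameplay Ability System.
; HandleCollision ignores itself, its owner and actors whose class is exactly BP_BaseWeapon.
; For any other actor it applies the passed-in effect if an Ability System Component is present, then destroys the projectile either way.
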(fn ConstructionScript)

(fn HandleCollision
  (params (Actor :type Actor%20Object%20Reference) (Effect :type Gameplay%20Effect%20Class%20Reference))
  (bind _returnvalue (Actor|GetComponentbyClass Actor "/Script/GameplayAbilities.AbilitySystemComponent"))
  (if (Math|Boolean|ANDBoolean (!= (Utilities|GetClass Actor) "/Game/_Game/Blueprints/Weapons/BP_BaseWeapon.BP_BaseWeapon_C") (!= Actor (Components|GetOwner)) (!= Actor self))
    (Utilities|IsValid _returnvalue
      (:Is%20Valid
        (GameplayEffects|ApplyGameplayEffectToSelf :self _returnvalue :GameplayEffectClass Effect)
        (Actor|DestroyActor))
      (:Is%20Not%20Valid
        (Actor|DestroyActor)))))